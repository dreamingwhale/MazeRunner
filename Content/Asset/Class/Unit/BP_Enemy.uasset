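; Enemy character Blueprint that tracks HP and dies when damage depletes it.
; AnyDamage subtracts from HP and, at zero or below, spawns an explosion emitter and calls OnDied, which destroys the actor and fires a death dispatcher.
; FnUpdateSpeed sets max walk speed, while FnMoveToPlayer is an empty stub with a disconnected movement node.
; Tick is empty, with a note to switch to interface-based communication.
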(event `self.ReceiveTick`
  (params (DeltaSeconds :type "Float (single-precision)"))
  ;[1 1 1] 틱이 아닌 인터페이스를 이용하여 통신하도록 수정 필요
)

(event `self.ReceiveAnyDamage`
  (params (Damage :type "Float (single-precision)") (DamageType :type "DamageType Object Reference") (InstigatedBy :type "Controller Object Reference") (DamageCauser :type "Actor Object Reference"))
  (bind _output_get (set `self.HP` (- (`self.HP`) Damage)))
  (if (<= _output_get 0.0)
    (`GameplayStatics.SpawnEmitterAtLocation` "/Game/StarterContent/Particles/P_Explosion.P_Explosion" (`self.K2_GetActorLocation` self))
    (`self.On Died`)))

(event `On Died`
  (`self.K2_DestroyActor`)
  (`self.OnDiedDispatcher`))

(fn `FnMoveToPlayer`)

(fn `FnUpdateSpeed`
  (params (InputSpeed :type "Float (double-precision)"))
  (set `CharacterMovementComponent.MaxWalkSpeed` InputSpeed (`self.CharacterMovement`)))

(fn `UserConstructionScript`)