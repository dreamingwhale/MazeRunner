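; Player pawn with hitscan shooting, a rough grenade action on G and contact combat against BP_Enemy.
; Left click line-traces forward from the camera manager and damages the hit actor.
; G spawns an FS_MasterField at the world origin, adding a projectile movement component for one swept move.
; Mesh overlap with an enemy subtracts its Attack from HP and damages it back; the FnTakeDamage hook is empty.
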(event `Key|LeftMouseButton`
  (params (Key :type "Key Structure"))
  (bind _returnvalue (`GameplayStatics.GetPlayerCameraManager` 0))
  (bind _returnvalue_2 (`self.K2_GetActorLocation` _returnvalue))
  ;[1 1 1] Shot
  (:`Pressed`
    (bind _outhit (`KismetSystemLibrary.LineTraceSingle` :`Start` _returnvalue_2 :`End` (+ _returnvalue_2 (* (`KismetMathLibrary.GetForwardVector` (`self.K2_GetActorRotation` _returnvalue)) 1000.0)) :`TraceChannel` "TraceTypeQuery1" :`DrawDebugType` "ForDuration"))
    (`GameplayStatics.ApplyDamage` (`.HitActor` (`GameplayStatics.BreakHitResult` _outhit)) 50.0)
    (`self.FnTakeDamage`)))

(event `Key|G`
  (params (Key :type "Key Structure"))
  ;[1 1 1] 수류탄
  (:`Pressed`
    (bind _returnvalue (`|SpawnActorFromClass` "/Engine/EditorResources/FieldNodes/FS_MasterField.FS_MasterField_C" (`KismetMathLibrary.MakeTransform` (0.0 0.0 0.0)) "Undefined" "MultiplyWithRoot" null null))
    (bind _returnvalue_2 (`AddComponent|NODE_AddProjectileMovementComponent-0` :`self` _returnvalue))
    (`MovementComponent.K2_MoveUpdatedComponent` :`self` _returnvalue_2 :`Delta` (100.0 100.0 0.0))))

(event `/Game/Asset/Interface/ClassInterface/IF_Enemy.FnTakeDamage`)

(event `OnActorBeginOverlap_Event`
  (params (OverlappedActor :type "Actor Object Reference") (OtherActor :type "Actor Object Reference"))
  (`KismetSystemLibrary.PrintString` (`KismetSystemLibrary.GetDisplayName` OtherActor)))

(event `self.MeshComponent.OnComponentBeginOverlap`
  (params (OverlappedComponent :type "PrimitiveComponent Object Reference") (OtherActor :type "Actor Object Reference") (OtherComp :type "PrimitiveComponent Object Reference") (OtherBodyIndex :type Integer) (bFromSweep :type Boolean) (SweepResult :type "HitResult Structure (by ref)"))
  (bind _asbp_enemy (cast `/Game/Asset/Class/Unit/BP_Enemy` OtherActor))
  (set `self.HP` (- (`self.HP`) (`/Game/Asset/Class/Unit/BP_Enemy.Attack` _asbp_enemy)))
  (`GameplayStatics.ApplyDamage` _asbp_enemy 200.0)
  (`self.FnTakeDamage`))

(fn `UserConstructionScript`)