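; BP_Grenades is a timed grenade actor that explodes three seconds after BeginPlay.
; A custom event spawns a BP_MasterField actor at the static mesh's transform and plays an explosion particle effect at its location.
; The grenade destroys itself after a short delay, with overlap, tick and construction logic left empty.
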(event `self.ReceiveBeginPlay`
  (`KismetSystemLibrary.Delay` 3.0)
  (`self.EventOnDestroied`))

(event `EventOnDestroied`
  (`|SpawnActorFromClass` "/Game/Asset/BluePrint/BP_MasterField.BP_MasterField_C" (`SceneComponent.K2_GetComponentToWorld` (`self.StaticMesh`)) "AlwaysSpawn" "MultiplyWithRoot" null null)
  (`GameplayStatics.SpawnEmitterAtLocation` "/Game/StarterContent/Particles/P_Explosion.P_Explosion" (`SceneComponent.K2_GetComponentLocation` (`self.StaticMesh`)))
  (`KismetSystemLibrary.Delay` 0.2)
  (`self.K2_DestroyActor`))

(fn `UserConstructionScript`)